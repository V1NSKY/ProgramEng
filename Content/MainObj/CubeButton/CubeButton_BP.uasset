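; Pressure button Blueprint that opens a linked double sliding CubeDoor while pressed, intended for BP_CubeF cubes.
; Box overlaps update an occupant counter and cast-check the actor, printing debug messages for non-cubes or a button already in use.
; The UpDown timeline moves the button and, on each update, plays or reverses the Door timeline according to IsPush, sliding both door halves.
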(event `self.Box.OnComponentBeginOverlap`
  (params (OverlappedComponent :type "PrimitiveComponent Object Reference") (OtherActor :type "Actor Object Reference") (OtherComp :type "PrimitiveComponent Object Reference") (OtherBodyIndex :type Integer) (bFromSweep :type Boolean) (SweepResult :type "HitResult Structure (by ref)"))
  (bind _cubedoor (`self.CubeDoor`))
  ;[1 1 1] In use or not
  (bind _result (`/Engine/EditorBlueprintResources/StandardMacros.IncrementInt` (`self.OWactors`))
    (:`  `
      (bind _output_get (set `self.OWactors` _result))
      (if (not (== _output_get 1))
        (`KismetSystemLibrary.PrintString` "Already in use" :!label _label))
      (cast `/Game/MainObj/Cube/BP_CubeF` OtherActor
        (:`then`
          _)
        (:`CastFailed`
          (`KismetSystemLibrary.PrintString` "Not Cube")))
      (set `self.IsPush` true)
      (bind (_direction _buttonupdown) (`Timeline|UpDown` :!label _label_2)
        (:`Update`
          (`SceneComponent.K2_SetRelativeLocation` (`self.Button`) (`KismetMathLibrary.MakeVector` 0.0 _buttonupdown) false false)
          (if (`self.IsPush`)
            (bind (_direction_2 _doorl _doorr) (`Timeline|Door` :!label _label_3)
              (:`Update`
                (`SceneComponent.K2_SetRelativeLocation` (`/Game/MainObj/Door/ButtonDoor_BP.DoorL` _cubedoor) (`KismetMathLibrary.MakeVector` 0.0 _doorl) false false)
                (`SceneComponent.K2_SetRelativeLocation` (`/Game/MainObj/Door/ButtonDoor_BP.DoorR` _cubedoor) (`KismetMathLibrary.MakeVector` 0.0 _doorr) false false)))
            (else
              (goto _label_3 :!via `Reverse`))))))))

(event `self.Box.OnComponentEndOverlap`
  (params (OverlappedComponent :type "PrimitiveComponent Object Reference") (OtherActor :type "Actor Object Reference") (OtherComp :type "PrimitiveComponent Object Reference") (OtherBodyIndex :type Integer))
  ;[1 1 1] In use or not
  (bind _result (`/Engine/EditorBlueprintResources/StandardMacros.DecrementInt` (`self.OWactors`))
    (:`  `
      (bind _output_get (set `self.OWactors` _result))
      (if (== _output_get 0)
        (cast `/Game/MainObj/Cube/BP_CubeF` OtherActor
          (:`then`
            _)
          (:`CastFailed`
            (`KismetSystemLibrary.PrintString` "Not Cube")))
        (set `self.IsPush` false)
        (goto _label_2 :!via `Reverse`)
        (else
          (goto _label))))))

(fn `UserConstructionScript`)