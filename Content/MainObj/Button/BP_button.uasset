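; Interactable button that toggles a linked DoorOnClick_BP sliding double door open and closed.
; Interact flips the open state, messages SecondDoor, then plays a button-press timeline that drives the door timeline forward or in reverse.
; A separate SecondButton event flips the state with opposite FlipFlop order and updates only the indicator.
; The indicator turns green or red through the spotlight and a newly created dynamic material instance.
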(event `/Game/Blueprints/Interfaces.Interact`
  (`/Engine/EditorBlueprintResources/StandardMacros.FlipFlop`
    (:`A`
      (set `self.FB_IsOpen` true))
    (:`B`
      (set `self.FB_IsOpen` false)))
  (message `/Game/Blueprints/Interfaces.SecondButton` (`self.SecondDoor`))
  (`self.OpenDoor`))

(event `/Game/Blueprints/Interfaces.SecondButton`
  (`/Engine/EditorBlueprintResources/StandardMacros.FlipFlop`
    (:`A`
      (set `self.FB_IsOpen` false))
    (:`B`
      (set `self.FB_IsOpen` true)))
  (`self.FB_ChangeLight` (`self.FB_IsOpen`)))

(event `OpenDoor`
  (bind _asdoor_on_click_bp (cast `/Game/MainObj/Door/DoorOnClick_BP` (`self.FB_Door`))
    (:`then`
      (`self.FB_ChangeLight` (`self.FB_IsOpen`))
      (bind (_direction _buttonclick) (`Timeline|ButtonClick` :!label _label)
        (:`Update`
          (`SceneComponent.K2_SetRelativeLocation` (`self.Button`) (`KismetMathLibrary.MakeVector` _buttonclick) false false)
          (if (`self.FB_IsOpen`)
            (bind (_direction_2 _doorr _doorl) (`Timeline|Door open` :`NewTime` 2.0 :!label _label_2)
              (:`Update`
                (`SceneComponent.K2_SetRelativeLocation` (`/Game/MainObj/Door/DoorOnClick_BP.DoorL` _asdoor_on_click_bp) (`KismetMathLibrary.MakeVector` 0.0 _doorl) false false)
                (`SceneComponent.K2_SetRelativeLocation` (`/Game/MainObj/Door/DoorOnClick_BP.DoorR` _asdoor_on_click_bp) (`KismetMathLibrary.MakeVector` 0.0 _doorr) false false)))
            (else
              (goto _label_2 :!via `Reverse`))))
        (:`Finished`
          (if (== _buttonclick 1.0)
            (goto _label :!via `Reverse`)))))
    (:`CastFailed`
      (`KismetSystemLibrary.PrintString` "Door not casted"))))

(fn `FB_ChangeLight`
  (params (IsOpen :type Boolean))
  (bind _spotlight (`self.SpotLight`))
  (bind _materialinst (`self.MaterialInst`))
  (bind _materialinst_2 (`self.MaterialInst`))
  (bind _buttonlight (`self.ButtonLight`))
  (if IsOpen
    (bind _output_get (set `self.FB_Color` (struct :`G` 1.0 :`A` 1.0)))
    (`LightComponent.SetLightColor` _spotlight _output_get true)
    (bind _output_get_2 (set `self.FB_Volume` 100.0))
    (bind _returnvalue (`PrimitiveComponent.CreateDynamicMaterialInstance` _buttonlight 0 "/Game/MainObj/Materials/LightRed.LightRed" "None"))
    (set `self.MaterialInst` _returnvalue)
    (`MaterialInstanceDynamic.SetVectorParameterValue` _materialinst_2 "Colour" _output_get)
    (`MaterialInstanceDynamic.SetScalarParameterValue` _materialinst_2 "Volume" _output_get_2)
    (else
      (bind _output_get_3 (set `self.FB_Color` (struct :`R` 1.0 :`A` 1.0)))
      (`LightComponent.SetLightColor` _spotlight _output_get_3 true)
      (bind _output_get_4 (set `self.FB_Volume` 100.0))
      (bind _returnvalue_2 (`PrimitiveComponent.CreateDynamicMaterialInstance` _buttonlight 0 "/Game/MainObj/Materials/LightRed.LightRed" "None"))
      (set `self.MaterialInst` _returnvalue_2)
      (`MaterialInstanceDynamic.SetVectorParameterValue` _materialinst "Colour" _output_get_3)
      (`MaterialInstanceDynamic.SetScalarParameterValue` _materialinst "Volume" _output_get_4))))

(fn `UserConstructionScript`)