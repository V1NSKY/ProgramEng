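; Door frame Blueprint with a door that the player toggles with E while standing in its trigger box.
; Overlap with the ThirdPersonCharacter enables or disables input, and the DoorOpen timeline plays or reverses to drive the door's relative Y location.
; A second box stops the timeline while a BPcube blocks it and reverses it when the cube leaves.
; Leaving the trigger also starts a timer whose event is empty.
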(event `self.Box.OnComponentBeginOverlap`
  (params (OverlappedComponent :type "PrimitiveComponent Object Reference") (OtherActor :type "Actor Object Reference") (OtherComp :type "PrimitiveComponent Object Reference") (OtherBodyIndex :type Integer) (bFromSweep :type Boolean) (SweepResult :type "HitResult Structure (by ref)"))
  (cast `/Game/ThirdPersonBP/Blueprints/ThirdPersonCharacter` OtherActor
    (:`then`
      (`self.EnableInput` (`GameplayStatics.GetPlayerController` 0)))
    (:`CastFailed`
      (`KismetSystemLibrary.PrintString` "Not a character"))))

(event `Key|E`
  (params (Key :type "Key Structure"))
  (:`Pressed`
    (if (< (stale _newtrack_0) 1.0)
      (bind (_direction _newtrack_0) (`Timeline|DoorOpen` :!label _label)
        (:`Update`
          (set `self.NewVar_0` _newtrack_0)
          (`SceneComponent.K2_SetRelativeLocation` (`self.Door`) (`KismetMathLibrary.MakeVector` 0.0 _newtrack_0) false false)))
      (else
        (goto _label :!via `Reverse`)))))

(event `self.Box.OnComponentEndOverlap`
  (params (OverlappedComponent :type "PrimitiveComponent Object Reference") (OtherActor :type "Actor Object Reference") (OtherComp :type "PrimitiveComponent Object Reference") (OtherBodyIndex :type Integer))
  (cast `/Game/ThirdPersonBP/Blueprints/ThirdPersonCharacter` OtherActor
    (:`then`
      (`self.DisableInput` (`GameplayStatics.GetPlayerController` 0))
      (`KismetSystemLibrary.K2_SetTimerDelegate` (delegate `Timer`) 3.0))
    (:`CastFailed`
      (`KismetSystemLibrary.PrintString` "Not character end overlap"))))

(event `Timer`)

(event `self.Box1.OnComponentBeginOverlap`
  (params (OverlappedComponent :type "PrimitiveComponent Object Reference") (OtherActor :type "Actor Object Reference") (OtherComp :type "PrimitiveComponent Object Reference") (OtherBodyIndex :type Integer) (bFromSweep :type Boolean) (SweepResult :type "HitResult Structure (by ref)"))
  (cast `/Game/Geometry/BPcube` OtherActor)
  (`KismetSystemLibrary.PrintString` "Block")
  (goto _label :!via `Stop`))

(event `self.Box1.OnComponentEndOverlap`
  (params (OverlappedComponent :type "PrimitiveComponent Object Reference") (OtherActor :type "Actor Object Reference") (OtherComp :type "PrimitiveComponent Object Reference") (OtherBodyIndex :type Integer))
  (cast `/Game/Geometry/BPcube` OtherActor)
  (`KismetSystemLibrary.PrintString` "Unblock")
  (goto _label :!via `Reverse`))

(fn `UserConstructionScript`)